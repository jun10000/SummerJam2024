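; Blueprint function library of game-wide helpers for typed pawn, controller and game instance lookups, transform reflection, texture size and UI display.
; The Show functions fetch singleton widgets from the game instance for game start, fade, timed hint, jigsaw puzzle and game clear screens.
; Interactive screens switch to UI-only input with a visible cursor through SetControllerInputMode.
; Game clear also disables pawn movement and plays a jingle.
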(fn GetMyPawn
  (params (PlayerIndex :type Integer))
  (bind _returnvalue (Game|Player|GetPlayerPawn 0 PlayerIndex))
  (bind (_asbp_pawn _bsuccess) (Utilities|Casting|CastToBP_Pawn _returnvalue))
  (return _asbp_pawn _bsuccess))

(fn GetMyPlayerController
  (params (PlayerIndex :type Integer))
  (bind _returnvalue (Game|GetPlayerController 0 PlayerIndex))
  (bind (_asbp_player_controller _bsuccess) (Utilities|Casting|CastToBP_PlayerController _returnvalue))
  (return _asbp_player_controller _bsuccess))

(fn GetMyGameInstance
  (bind _returnvalue (Game|GetGameInstance))
  (bind (_asbp_game_instance _bsuccess) (Utilities|Casting|CastToBP_GameInstance _returnvalue))
  (return _asbp_game_instance _bsuccess))

(fn ReflectVector
  (params (InVec :type Vector) (X :type Boolean) (Y :type Boolean) (Z :type Boolean))
  (bind (_x _y _z) (Math|Vector|BreakVector InVec))
  (return (Math|Vector|MakeVector (* _x (Math|Float|SelectFloat -1.0 1.0 X)) (* _y (Math|Float|SelectFloat -1.0 1.0 Y)) (* _z (Math|Float|SelectFloat -1.0 1.0 Z)))))

(fn ReflectRotator
  (params (InRotator :type Rotator) (X%20%28Roll%29 :type Boolean) (Y%20%28Pitch%29 :type Boolean) (Z%20%28Yaw%29 :type Boolean))
  (bind (_roll _pitch _yaw) (Math|Rotator|BreakRotator InRotator))
  (return (Math|Rotator|MakeRotator (+ _roll (Math|Float|SelectFloat 1.8e+02 0.0 X%20%28Roll%29)) (+ _pitch (Math|Float|SelectFloat 1.8e+02 0.0 Y%20%28Pitch%29)) (+ _yaw (Math|Float|SelectFloat 1.8e+02 0.0 Z%20%28Yaw%29)))))

(fn ReflectTransform
  (params (InTransform :type Transform) (X :type Boolean) (Y :type Boolean) (Z :type Boolean) (Roll :type Boolean) (Pitch :type Boolean) (Yaw :type Boolean))
  (bind (_location _rotation _scale) (Math|Transform|BreakTransform InTransform))
  (return (Math|Transform|MakeTransform (CallFunction|ReflectVector _location X Y Z) (CallFunction|ReflectRotator _rotation Roll Pitch Yaw) _scale)))

(fn ShowGameStart
  (bind (_returnvalue _success) (CallFunction|GetMyGameInstance))
  (if _success
    (bind _asw_game_start (Utilities|Casting|CastToW_GameStart (Default|GetSingletonWidget _returnvalue "/Game/Widgets/W_GameStart.W_GameStart_C")))
    (UserInterface|Viewport|AddtoViewport _asw_game_start 0)
    (CallFunction|SetControllerInputMode "NewEnumerator1" 0 _asw_game_start)))

(fn ShowFadein
  (params (IsReverse :type Boolean))
  (bind (_returnvalue _success) (CallFunction|GetMyGameInstance))
  (if _success
    (bind _asw_fade (Utilities|Casting|CastToW_Fade (Default|GetSingletonWidget _returnvalue "/Game/Widgets/W_Fade.W_Fade_C")))
    (UserInterface|Viewport|AddtoViewport _asw_fade 0)
    (UserInterface|Animation|PlayAnimation _asw_fade (Variables|/Game/Widgets/W_Fade.W_Fade_C|GetFadeIn _asw_fade) 0.0 1 (select IsReverse "Reverse" "Forward") 1.0 false)))

(fn ShowHint
  (params (Text :type Text) (Duration :type Float%20%28single-precision%29))
  (bind (_returnvalue _success) (CallFunction|GetMyGameInstance))
  (if _success
    (bind _asw_hint (Utilities|Casting|CastToW_Hint (Default|GetSingletonWidget _returnvalue "/Game/Widgets/W_Hint.W_Hint_C")))
    (Variables|/Game/Widgets/W_Hint.W_Hint_C|SetHintText _asw_hint Text)
    (UserInterface|Viewport|AddtoViewport _asw_hint 0)
    (UserInterface|Animation|PlayAnimation _asw_hint (Variables|/Game/Widgets/W_Hint.W_Hint_C|GetShowAndHideAnimation _asw_hint) 0.0 1 "Forward" (Math|Float|SafeDivide 5.5 (+ Duration 0.5)) false)))

(fn GetTextureSize
  (params (Texture :type Texture%202D%20Object%20Reference))
  (return (Math|Vector2D|MakeVector2D (Math|Conversions|ToFloat(Integer) (Class|Texture2D|BlueprintGetSizeX Texture)) (Math|Conversions|ToFloat(Integer) (Class|Texture2D|BlueprintGetSizeY Texture)))))

(fn ShowJigsawPuzzle
  (params (OnClear :type Delegate%20%28by%20ref%29))
  (bind (_returnvalue _success) (CallFunction|GetMyGameInstance))
  (if _success
    (bind _asw_jigsaw_puzzle (Utilities|Casting|CastToW_JigsawPuzzle (Default|GetSingletonWidget _returnvalue "/Game/Widgets/W_JigsawPuzzle.W_JigsawPuzzle_C")))
    (UserInterface|Viewport|AddtoViewport _asw_jigsaw_puzzle 0)
    (CallFunction|SetControllerInputMode "NewEnumerator1" 0 _asw_jigsaw_puzzle)
    (EventDispatchers|UnbindallEventsfromOnClear _asw_jigsaw_puzzle)
    (EventDispatchers|BindEventtoOnClear _asw_jigsaw_puzzle OnClear)))

(fn ShowGameClear
  (params (EndingName :type Text) (Jingle :type Sound%20Base%20Object%20Reference))
  (bind (_returnvalue _success) (CallFunction|GetMyGameInstance))
  (bind (_returnvalue_2 _success_2) (デフォルト|GetMyPawn))
  (if _success_2
    (Pawn|Components|CharacterMovement|DisableMovement (Variables|/Script/Engine.Character|GetCharacterMovement _returnvalue_2))
    (if _success
      (bind _asw_game_clear (Utilities|Casting|CastToW_GameClear (Default|GetSingletonWidget _returnvalue "/Game/Widgets/W_GameClear.W_GameClear_C")))
      (UserInterface|Viewport|AddtoViewport _asw_game_clear 0)
      (Variables|/Game/Widgets/W_GameClear.W_GameClear_C|SetEndingName _asw_game_clear EndingName)
      (CallFunction|SetControllerInputMode "NewEnumerator1" 0 _asw_game_clear)
      (Audio|PlaySound2D 0 Jingle 1.0 1.0 0.0 0 0)
      (Class|UserWidget|PlayAnimationForward _asw_game_clear (Variables|/Game/Widgets/W_GameClear.W_GameClear_C|GetStartAnimation _asw_game_clear) 1.0 false))))

(fn SetControllerInputMode
  (params (Mode :type E_InputMode%20Enum :default "NewEnumerator0") (FocusWidget :type Widget%20Object%20Reference))
  (bind (_returnvalue _success) (CallFunction|GetMyPlayerController))
  (if _success
    (switch Utilities|FlowControl|Switch|SwitchonE_InputMode Mode
      (:NewEnumerator0
        (Input|SetInputModeGameOnly _returnvalue false)
        (Variables|/Script/Engine.PlayerController|SetbShowMouseCursor _returnvalue false))
      (:NewEnumerator1
        (Input|SetInputModeUIOnly _returnvalue FocusWidget "DoNotLock" false)
        (Variables|/Script/Engine.PlayerController|SetbShowMouseCursor _returnvalue true)))))