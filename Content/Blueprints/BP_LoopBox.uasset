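; BP_LoopBox is an overlap volume that traps BP_Pawn in a repeating stretch of space, sending it back to where it entered.
; When looping is enabled, the first overlap stores the entry location and resets the counter, with IsLooping guarding against re-entry.
; Exiting near the entry point cancels the loop.
; Exiting elsewhere moves the pawn back until MaxLoopCount is exceeded, then ends the loop and calls LoopFinished.
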(event EventBeginPlay)

(event Collision|EventActorBeginOverlap
  (params (OtherActor :type Actor%20Object%20Reference))
  (bind _asbp_pawn (Utilities|Casting|CastToBP_Pawn OtherActor))
  (bind _output_get (Variables|Temporary|SetCurrentPawn _asbp_pawn))
  (Variables|Temporary|SetCurrentLocation (Transformation|GetActorLocation _output_get))
  (if (and (Variables|Default|GetEnableLoop) (not (Variables|Default|GetIsLooping)))
    (Variables|Default|SetIsLooping true)
    (Variables|Default|SetEntriedLocation (Variables|Temporary|GetCurrentLocation))
    (Variables|Default|SetCurrentLoopCount 0)))

(event Collision|EventActorEndOverlap
  (params (OtherActor :type Actor%20Object%20Reference))
  (bind _asbp_pawn (Utilities|Casting|CastToBP_Pawn OtherActor))
  (bind _output_get (Variables|Temporary|SetCurrentPawn _asbp_pawn))
  (Variables|Temporary|SetCurrentLocation (Transformation|GetActorLocation _output_get))
  (if (and (Variables|Default|GetEnableLoop) (Variables|Default|GetIsLooping))
    (if (Utilities|Operators|EqualEqual (Variables|Temporary|GetCurrentLocation) (Variables|Default|GetEntriedLocation) (Variables|Default|GetLocationTolerance))
      (Variables|Default|SetIsLooping false)
      (else
        (bind _result (Math|Integer|IncrementInt (Variables|Default|GetCurrentLoopCount))
          (:%20%20
            (if (<= _result (Variables|Default|GetMaxLoopCount))
              (Transformation|SetActorLocation (Variables|Temporary|GetCurrentPawn) (Variables|Default|GetEntriedLocation) false false)
              (else
                (Variables|Default|SetIsLooping false)
                (Default|CallLoopFinished)))))))))

(fn ConstructionScript)