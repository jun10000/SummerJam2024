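; Player controller Blueprint that handles basic movement input for the possessed pawn.
; On BeginPlay it adds the default Enhanced Input mapping context.
; Forward and right input actions add movement input to the pawn along the current view target's forward and right vectors, so movement follows the view target's orientation rather than the pawn's.
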(event Input|EnhancedActionEvents|EnhancedInputActionIA_MoveForward
  (params (ActionValue :type Float%20%28double-precision%29) (ElapsedSeconds :type Float%20%28double-precision%29) (TriggeredSeconds :type Float%20%28double-precision%29) (InputAction :type Input%20Action%20Object%20Reference :default "/Game/Input/IA_MoveForward.IA_MoveForward"))
  (bind _returnvalue (Utilities|GetMyPawn)
    (:Success
      (Pawn|Input|AddMovementInput _returnvalue (Transformation|GetActorForwardVector (Pawn|GetViewTarget)) ActionValue false))))

(event Input|EnhancedActionEvents|EnhancedInputActionIA_MoveRight
  (params (ActionValue :type Float%20%28double-precision%29) (ElapsedSeconds :type Float%20%28double-precision%29) (TriggeredSeconds :type Float%20%28double-precision%29) (InputAction :type Input%20Action%20Object%20Reference :default "/Game/Input/IA_MoveRight.IA_MoveRight"))
  (bind _returnvalue (Utilities|GetMyPawn)
    (:Success
      (Pawn|Input|AddMovementInput _returnvalue (Transformation|GetActorRightVector (Pawn|GetViewTarget)) ActionValue false))))

(event EventBeginPlay
  (Input|AddMappingContext (PlayerController|LocalPlayerSubsystems|GetEnhancedInputLocalPlayerSubsystem self) "/Game/Input/IMC_Default.IMC_Default" 0 "(bIgnoreAllPressedKeysUntilRelease=True,bForceImmediately=False,bNotifyUserSettings=False)"))

(fn ConstructionScript)