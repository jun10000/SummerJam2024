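; BP_Switch_Push is a push switch with a configurable colored mesh and point light, which signals when it is triggered.
; The construction script applies the color, intensity and intensity units to the point light.
; On BeginPlay, it creates a dynamic material instance on the mesh and sets its color parameter to match.
; The Trig event fires the Pushed dispatcher only while the switch is triggerable.
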(event EventBeginPlay
  (bind _returnvalue (Rendering|Material|CreateDynamicMaterialInstance (Variables|Debug|GetStaticMeshComponent) 0 0 "None" :!class /Script/Engine.PrimitiveComponent))
  (bind _output_get (Variables|Default|SetDMI _returnvalue))
  (Rendering|Material|SetVectorParameterValue _output_get (Variables|Default|GetColorParameterName) (Variables|Default|GetColor) :!class /Script/Engine.MaterialInstanceDynamic))

(event EventTrig
  (if (Variables|Default|GetIsTriggerable)
    (Default|CallPushed)))

(fn ConstructionScript
  (bind _pointlight (Variables|Default|GetPointLight))
  (Rendering|Components|Light|SetLightColor _pointlight (Variables|Default|GetColor) true)
  (Rendering|Components|Light|SetIntensity _pointlight (Variables|Default|GetLightIntensity))
  (Class|LocalLightComponent|SetIntensityUnits _pointlight (Variables|Default|GetLightIntensityUnits)))